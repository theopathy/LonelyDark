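; Floating battle text actor, likely a damage number popup, that shows a given text in a given color, rises and then removes itself.
; On BeginPlay it applies Text and Color to its TextRender and shifts the actor along world Y.
; The slowed Fade timeline lerps the text's relative height from an offset based on the Y variable, then destroys the actor when finished.
; Despite its name, Fade only drives movement, not opacity.
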(event `self.ReceiveBeginPlay`
  (bind _y (`self.Y`))
  (`|ExecutionSequence`
    (:`then_0`
      (`TextRenderComponent.SetTextRenderColor` (`self.TextRender`) (`KismetMathLibrary.Conv_LinearColorToColor` (`self.Color`)))
      (`TextRenderComponent.K2_SetText` (`self.TextRender`) (`self.Text`))
      (`self.K2_AddActorWorldOffset` (0.0 350.0 0.0)))
    (:`then_1`
      (`TimelineComponent.SetPlayRate` (`self.fade`) 0.6)
      (bind (_direction _transparency _height) (`Timeline|fade`)
        (:`Update`
          (`SceneComponent.K2_SetRelativeLocation` (`self.TextRender`) (`KismetMathLibrary.MakeVector` -50.0 60.0 (`KismetMathLibrary.Lerp` (+ _y 85.0) (+ _y 125.0) _height)) false false))
        (:`Finished`
          (`self.K2_DestroyActor`))))))

(fn `UserConstructionScript`)